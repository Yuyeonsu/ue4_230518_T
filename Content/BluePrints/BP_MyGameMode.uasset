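; BP_MyGameMode is the game mode that runs the HUD, score and win/lose outcome.
; BeginPlay adds the player UI and sets game-only input, while AddScore triggers a clear GameResult at five points.
; Tick polls all BP_Light2 actors and sets Exploding when their count equals PassedLights.
; GameResult shows the clear or game-over widget and plays ResultCue with a bool parameter, whose name is left as None.
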(event `self.ReceiveBeginPlay`
  (bind _returnvalue (`GameplayStatics.GetPlayerController` 0))
  ;[1 1 1] 화면에 체력 바 표시
  (bind _returnvalue_2 (`|CreateWidget` "/Game/UMG/PlayerUI.PlayerUI_C"))
  (`UserWidget.AddToViewport` _returnvalue_2 0)
  (`/Engine/EditorBlueprintResources/StandardMacros.IsValid` _returnvalue
    (:`Is Valid`
      (`WidgetBlueprintLibrary.SetInputMode_GameOnly` _returnvalue))))

(event `self.ReceiveTick`
  (params (DeltaSeconds :type "Float (single-precision)"))
  ;[1 1 1] 폭발 이벤트
  (bind _outactors (`GameplayStatics.GetAllActorsOfClass` "/Game/BluePrints/BP_Light2.BP_Light2_C"))
  (bind _output_get (set `self.NumberOfLights` (`KismetArrayLibrary.Array_Length` _outactors)))
  (if (== _output_get (`self.PassedLights`))
    (set `self.Exploding` true)))

(event `GameResult`
  (params (Clear :type Boolean))
  ;[1 1 1] 게임 결과에 따라 위젯 표시 / 사운드 변경
  (bind _returnvalue (`|CreateWidget` (select `bool` Clear :`false` "/Game/UMG/GameOverUI.GameOverUI_C" :`true` "/Game/UMG/ClearUI.ClearUI_C" :!type "UserWidget Class Reference")))
  (set `self.ClearFlag` (select `bool` Clear :`true` true))
  (`UserWidget.AddToViewport` _returnvalue 0)
  (bind _returnvalue_2 (`GameplayStatics.SpawnSoundAtLocation` "/Game/Audio/ResultCue.ResultCue" (0.0 0.0 0.0) (struct) 1.0 1.0 0.0 null null))
  (`AudioComponent.SetBoolParameter` _returnvalue_2 "None" (`self.ClearFlag`)))

(fn `AddScore`
  (bind _output_get (set `self.TotalScore` (+ (`self.TotalScore`) 1)))
  ;[1 1 1] clear 조건 설정
  (if (>= _output_get 5)
    (`self.GameResult` true)))

(fn `UserConstructionScript`)